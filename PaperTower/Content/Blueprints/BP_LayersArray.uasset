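; BP_LayersArray is a 2D container for terrain cubes, stored in a flat LayerArray.
; Init sets both dimensions, then clears and resizes the array to their product.
; Get and set map coordinates through ArrayIndexFromDimensions as D1 * D1Size + D2, a stride that suits only square grids.
; That helper checks only the upper bound of the flat index and prints a message when exceeded.
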(fn `ArrayIndexFromDimensions`
  (params (d1 :type Integer) (d2 :type Integer))
  (returns (index :type Integer))
  (bind _returnvalue (+ (* d1 (`self.d1Size`)) d2))
  (if (< _returnvalue (`KismetArrayLibrary.Array_Length` (`self.layerArray`)))
    (return _returnvalue)
    (else
      (`KismetSystemLibrary.PrintString` "index out of bounds" true true (struct :`G` 0.66 :`B` 1.0 :`A` 1.0) 10.0))))

(fn `GetElement2D`
  (params (d1 :type Integer) (d2 :type Integer))
  (returns (terrainObject :type "/Game/Blueprints/Layers/BP_TerrainCube Object Reference"))
  (return (`|GetArrayItem` (`self.layerArray`) (`self.ArrayIndexFromDimensions` d1 d2))))

(fn `Init`
  (params (d1SizeIn :type Integer) (d2SizeIn :type Integer))
  (bind _layerarray (`self.layerArray`))
  (set `self.d1Size` d1SizeIn)
  (set `self.d2Size` d2SizeIn)
  (bind _output_get (set `self.arraySize` (* (`self.d1Size`) (`self.d2Size`))))
  (`KismetArrayLibrary.Array_Clear` _layerarray)
  (`KismetArrayLibrary.Array_Resize` _layerarray _output_get))

(fn `SetElement2D`
  (params (d1 :type Integer) (d2 :type Integer) (terrainCube :type "/Game/Blueprints/Layers/BP_TerrainCube Object Reference"))
  (`KismetArrayLibrary.Array_Set` (`self.layerArray`) (`self.ArrayIndexFromDimensions` d1 d2) terrainCube))

(fn `UserConstructionScript`)