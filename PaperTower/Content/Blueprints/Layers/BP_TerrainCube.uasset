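; BP_TerrainCube is a mineable terrain block in a clicker game, damaged by player clicks or miner hits while active.
; Clicks subtract multiplied click power, while miners pass in new health; each hit shrinks the cube by a step derived from max health and unmultiplied power.
; At zero health it pays money, may yield its material, updates the UI, destroys itself and advances the GameState's layer count logic.
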(event `self.ReceiveBeginPlay`
  (bind _asbp_clicker_player (cast `/Game/Blueprints/BP_ClickerPlayer` (`GameplayStatics.GetPlayerCharacter` 0)))
  (set `self.player` _asbp_clicker_player)
  (bind _asbp_paper_tower_game_state (cast `/Game/Blueprints/BP_PaperTowerGameState` (`GameplayStatics.GetGameState`)))
  (set `self.gameState` _asbp_paper_tower_game_state)
  (`self.findCubeSizeDecrement` 0)
  (set `self.currentHealth` (`self.maxHealth`)))

(event `minerHit`
  (params (newHealth :type Integer) (power :type Integer))
  (bind _gamestate (`self.gameState`))
  (bind _cube (`self.Cube`))
  (bind _player (`self.player`))
  (bind _player_2 (`self.player`))
  (bind _player_3 (`self.player`))
  (bind _returnvalue (`KismetMathLibrary.RandomIntegerInRange` (`self.yieldMin`) (`self.yieldMax`)))
  (bind _ui_ref (`/Game/Blueprints/BP_ClickerPlayer.UI Ref` _player_2))
  (if (`self.isActive`)
    (set `self.currentHealth` newHealth)
    (`self.findCubeSizeDecrement` power)
    (if (<= (`self.currentHealth`) 0) :!label _label
      (set `/Game/Blueprints/BP_ClickerPlayer.money` (+ (`self.moneyValue`) (`/Game/Blueprints/BP_ClickerPlayer.money` _player_3)) _player_3)
      (`/Game/Blueprints/WBP_MainUI.Update Money Text` (`/Game/Blueprints/BP_ClickerPlayer.UI Ref` (`self.player`)))
      (if (> (`KismetMathLibrary.RandomFloatInRange` 0.0 1.0) (`self.yieldChance`))
        (`self.K2_DestroyActor`)
        (else
          (switch `/Game/Blueprints/E_MaterialTypes` (`self.materialType`)
            (:`NewEnumerator0`
              (set `/Game/Blueprints/BP_ClickerPlayer.stoneInventory` (+ (`/Game/Blueprints/BP_ClickerPlayer.stoneInventory` _player) _returnvalue) _player_2)
              (`/Game/Blueprints/WBP_MainUI.Update Stone Text` _ui_ref))
            (:`NewEnumerator1`
              (set `/Game/Blueprints/BP_ClickerPlayer.ironInventory` (+ (`/Game/Blueprints/BP_ClickerPlayer.ironInventory` _player) _returnvalue) _player_2)
              (`/Game/Blueprints/WBP_MainUI.Update Iron Text` _ui_ref))
            (:`NewEnumerator2`
              (set `/Game/Blueprints/BP_ClickerPlayer.gemInventory` (+ (`/Game/Blueprints/BP_ClickerPlayer.gemInventory` _player) _returnvalue) _player_2)
              (`/Game/Blueprints/WBP_MainUI.Update Gem Text` _ui_ref))
            (:`NewEnumerator3`
              (set `/Game/Blueprints/BP_ClickerPlayer.obsidianInventory` (+ (`/Game/Blueprints/BP_ClickerPlayer.obsidianInventory` _player) _returnvalue) _player_2)
              (`/Game/Blueprints/WBP_MainUI.Update Obsidian Text` _ui_ref)))
          (`self.K2_DestroyActor`)))
      (`/Engine/EditorBlueprintResources/StandardMacros.DecrementInt` (`/Game/Blueprints/BP_PaperTowerGameState.currentLayerCount` _gamestate)
        (:`  `
          (`/Game/Blueprints/BP_PaperTowerGameState.incrementLayer` _gamestate)))
      (else
        (`SceneComponent.SetRelativeScale3D` _cube (- (`SceneComponent.RelativeScale3D` _cube) (`self.cubeSizeDecrementAmount`)))))))

(event `self.ClickBox.OnClicked`
  (params (TouchedComponent :type "PrimitiveComponent Object Reference") (ButtonPressed :type "Key Structure"))
  (bind _player (`self.player`))
  (if (`self.isActive`)
    (set `self.currentHealth` (`KismetMathLibrary.FTrunc` (- (`self.currentHealth`) (* (`/Game/Blueprints/BP_ClickerPlayer.clickPower` _player) (`/Game/Blueprints/BP_ClickerPlayer.currentMultiplier` _player)))))
    (`self.findCubeSizeDecrement` (`/Game/Blueprints/BP_ClickerPlayer.clickPower` (`self.player`)))
    (goto _label)))

(fn `findCubeSizeDecrement`
  (params (power :type Integer))
  (set `self.cubeSizeDecrementAmount` (/ (`SceneComponent.RelativeScale3D` (`self.ClickBox`)) (`KismetMathLibrary.FCeil` (`KismetMathLibrary.SafeDivide` (`KismetMathLibrary.Conv_IntToDouble` (`self.maxHealth`)) (`KismetMathLibrary.Conv_IntToDouble` power))))))

(fn `UserConstructionScript`)