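; BP_Miner is an autonomous miner that seeks out and damages objects on the current layer of the paper tower in a clicker game.
; Tick runs a three-state machine on HasTarget: select, travel, then hit after each Rest delay.
; Selection takes a random object from the GameState's current layer array and removes that entry.
; It flies straight to a point above the target without sweeping, and reselects once the target is invalid.
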(event `self.ReceiveBeginPlay`
  (bind _asbp_clicker_player (cast `/Game/Blueprints/BP_ClickerPlayer` (`GameplayStatics.GetPlayerCharacter` 0)))
  (set `self.Player` _asbp_clicker_player)
  (bind _asbp_paper_tower_game_state (cast `/Game/Blueprints/BP_PaperTowerGameState` (`GameplayStatics.GetGameState`)))
  (set `self.Game State` _asbp_paper_tower_game_state))

(event `select target`
  (bind _game_state (`self.Game State`))
  (switch `int` (- (`/Game/Blueprints/BP_PaperTowerGameState.currentLayer` (`self.Game State`)) 1)
    (:`0`
      (`self.setTarget` (`/Game/Blueprints/BP_PaperTowerGameState.layer1objects` _game_state)))
    (:`1`
      (`self.setTarget` (`/Game/Blueprints/BP_PaperTowerGameState.layer2objects` _game_state)))
    (:`2`
      (`self.setTarget` (`/Game/Blueprints/BP_PaperTowerGameState.layer3objects` _game_state)))
    (:`3`
      (`self.setTarget` (`/Game/Blueprints/BP_PaperTowerGameState.layer4objects` _game_state)))
    (:`4`
      (`self.setTarget` (`/Game/Blueprints/BP_PaperTowerGameState.layer5objects` _game_state)))))

(event `self.ReceiveTick`
  (params (DeltaSeconds :type "Float (single-precision)"))
  (bind _returnvalue (`self.K2_GetActorLocation`))
  (bind _target (`self.target`))
  (bind _targetlocation (`self.targetLocation`))
  (switch `int` (`self.hasTarget`)
    (:`0`
      (`self.select target`))
    (:`1`
      (if (`KismetSystemLibrary.IsValid` (`self.target`))
        (bind _out (`self.incrementDistance` _targetlocation _returnvalue DeltaSeconds))
        (`self.K2_SetActorLocation` _out)
        (if (== _targetlocation _returnvalue :`ErrorTolerance` 1.0)
          (set `self.hasTarget` 2))
        (else
          (set `self.hasTarget` 0))))
    (:`2`
      (`KismetSystemLibrary.Delay` (`self.rest`))
      (if (`KismetSystemLibrary.IsValid` (`self.target`))
        (`/Game/Blueprints/Layers/BP_TerrainCube.minerHit` _target (`KismetMathLibrary.FTrunc` (- (`/Game/Blueprints/Layers/BP_TerrainCube.currentHealth` _target) (`self.damage`))) (`KismetMathLibrary.FTrunc` (`self.damage`)))
        (else
          (set `self.hasTarget` 0))))))

(fn `incrementDistance`
  (params (targetPos :type "Vector Structure") (curPos :type "Vector Structure") (deltaTime :type "Float (double-precision)"))
  (returns (out :type "Vector Structure"))
  (return (+ curPos (* (`KismetMathLibrary.Normal` (- targetPos curPos)) (* deltaTime (`self.speed`))))))

(fn `setTarget`
  (params (layerArray :type "Array of /Game/Blueprints/Layers/BP_TerrainCube Object Reference"))
  (locals (randomInt :type Integer))
  (bind _returnvalue_location (`KismetMathLibrary.BreakTransform` (`self.GetTransform` (`self.target`))))
  (bind _output_get (set `local.randomInt` (`KismetMathLibrary.RandomIntegerInRange` 0 (- (`KismetArrayLibrary.Array_Length` layerArray) 1))))
  (set `self.target` (`|GetArrayItem` layerArray _output_get))
  (`KismetArrayLibrary.Array_Remove` layerArray (`local.randomInt`))
  (set `self.targetLocation` (+ _returnvalue_location (0.0 0.0 100.0)))
  (set `self.hasTarget` 1))

(fn `UserConstructionScript`)