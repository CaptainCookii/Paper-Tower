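; BP_TerrainCube is a clickable cube that awards money to the player when clicking destroys it.
; On BeginPlay it caches the clicker player and game state, then derives a shrink step from its scale divided by Health.
; Each click subtracts click power times multiplier from Health and shrinks the cube by that fixed step, whatever the damage.
; At zero Health it adds MoneyValue to the player's Money and destroys itself.
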(event `self.ReceiveBeginPlay`
  (bind _asbp_clicker_player (cast `/Game/Blueprints/BP_ClickerPlayer` (`GameplayStatics.GetPlayerCharacter` 0)))
  (set `self.player` _asbp_clicker_player)
  (bind _asbp_paper_tower_game_state (cast `/Game/Blueprints/BP_PaperTowerGameState` (`GameplayStatics.GetGameState`)))
  (set `self.gameState` _asbp_paper_tower_game_state)
  (set `self.cubeSizeDecrementAmount` (/ (`SceneComponent.RelativeScale3D` (`self.Cube`)) (`self.health`))))

(event `self.Cube.OnClicked`
  (params (TouchedComponent :type "PrimitiveComponent Object Reference") (ButtonPressed :type "Key Structure"))
  (bind _player (`self.player`))
  (bind _cube (`self.Cube`))
  (bind _player_2 (`self.player`))
  (bind _returnvalue (+ (`self.moneyValue`) (`/Game/Blueprints/BP_ClickerPlayer.money` _player_2)))
  (bind _output_get (set `self.health` (`KismetMathLibrary.FTrunc` (- (`self.health`) (* (`/Game/Blueprints/BP_ClickerPlayer.clickPower` _player) (`/Game/Blueprints/BP_ClickerPlayer.currentMultiplier` _player))))))
  (if (<= _output_get 0)
    (set `/Game/Blueprints/BP_ClickerPlayer.money` _returnvalue _player_2)
    (`KismetSystemLibrary.PrintString` (`KismetStringLibrary.Conv_IntToString` _returnvalue))
    (`self.K2_DestroyActor`)
    (else
      (`SceneComponent.SetRelativeScale3D` _cube (- (`SceneComponent.RelativeScale3D` _cube) (`self.cubeSizeDecrementAmount`))))))

(fn `UserConstructionScript`)