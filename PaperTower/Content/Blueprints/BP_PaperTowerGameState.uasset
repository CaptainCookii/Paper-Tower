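; Game state for a clicker mining game that owns the layered cube world and the roster of AI miners.
; CreateWorld fills a 2D TerrainLayers actor with 20 stacked 5x5 layers, each using its own cube class.
; IncrementLayer activates the next layer once the current count empties, moves the player and clears miner targets, rebuilding the world after the last.
; SpawnMiner and update events copy the player's damage, speed and rest stats to miners.
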(event `self.ReceiveBeginPlay`
  (bind _returnvalue (`GameplayStatics.GetPlayerController` 0))
  (set `PlayerController.bShowMouseCursor` true _returnvalue)
  (set `PlayerController.bEnableClickEvents` true _returnvalue)
  (`WidgetBlueprintLibrary.SetInputMode_GameAndUIEx` _returnvalue null)
  (bind _asbp_clicker_player (cast `/Game/Blueprints/BP_ClickerPlayer` (`GameplayStatics.GetPlayerCharacter` 0)))
  (set `self.Player` _asbp_clicker_player)
  (bind _returnvalue_2 (`GameplayStatics.GetActorOfClass` "/Game/Blueprints/BP_LayersArray.BP_LayersArray_C"))
  (set `self.terrainLayers` _returnvalue_2)
  (`self.createWorld`))

(event `incrementLayer`
  (bind _d2size (`/Game/Blueprints/BP_LayersArray.d2Size` (`self.terrainLayers`)))
  (if (<= (`self.currentLayerCount`) 0)
    (bind _result (`/Engine/EditorBlueprintResources/StandardMacros.IncrementInt` (`self.currentLayer`))
      (:`  `
        (if (> _result (`/Game/Blueprints/BP_LayersArray.d1Size` (`self.terrainLayers`)))
          (`self.createWorld`)
          (else
            (set `self.currentLayerCount` _d2size)
            (set `self.numValidCount` _d2size)
            (bind _returnvalue (- _result 1))
            (`self.activateLayer` _returnvalue)
            (bind _terrainobject (`/Game/Blueprints/BP_LayersArray.GetElement2D` (`self.terrainLayers`) _returnvalue 0))
            (`self.K2_SetActorLocation` (`self.Player`) (- (`self.K2_GetActorLocation` _terrainobject) (300.0 230.0 -300.0)) false false)
            (for _array_element (`self.minersArray`)
              (set `/Game/Blueprints/BP_Miner.hasTarget` 0 _array_element))))))))

(event `createWorld`
  (bind _minersarray (`self.minersArray`))
  (bind _d2size (`/Game/Blueprints/BP_LayersArray.d2Size` (`self.terrainLayers`)))
  (`/Game/Blueprints/BP_LayersArray.Init` (`self.terrainLayers`) 20 25)
  (`self.generateLayers`)
  (set `self.currentLayer` 1)
  (set `self.currentLayerCount` _d2size)
  (set `self.numValidCount` _d2size)
  (if (`KismetArrayLibrary.Array_IsNotEmpty` _minersarray)
    (for _array_element _minersarray
      (`self.K2_SetActorLocation` _array_element (400.0 400.0 2100.0) false true)
      (bind _terrainobject (`/Game/Blueprints/BP_LayersArray.GetElement2D` (`self.terrainLayers`) 0 0))
      (`self.K2_SetActorLocation` (`self.Player`) (- (`self.K2_GetActorLocation` _terrainobject) (300.0 230.0 -300.0)) false false))))

(event `spawnMiner`
  (bind _player (`self.Player`))
  (bind _returnvalue (`|SpawnActorFromClass` "/Game/Blueprints/BP_Miner.BP_Miner_C" (`KismetMathLibrary.MakeTransform` (`KismetMathLibrary.MakeVector` 400.0 400.0 (`KismetMathLibrary.Conv_IntToDouble` (- 2200 (* (`self.currentLayer`) 100))))) "Undefined" "MultiplyWithRoot" null null))
  (`KismetArrayLibrary.Array_Add` (`self.minersArray`) _returnvalue)
  (set `/Game/Blueprints/BP_Miner.damage` (`/Game/Blueprints/BP_ClickerPlayer.minerDmg` _player) _returnvalue)
  (set `/Game/Blueprints/BP_Miner.speed` (`/Game/Blueprints/BP_ClickerPlayer.minerSpeed` _player) _returnvalue)
  (set `/Game/Blueprints/BP_Miner.rest` (`/Game/Blueprints/BP_ClickerPlayer.minerRest` _player) _returnvalue))

(event `updateMinerDmg`
  (for _array_element (`self.minersArray`)
    (set `/Game/Blueprints/BP_Miner.damage` (`/Game/Blueprints/BP_ClickerPlayer.minerDmg` (`self.Player`)) _array_element)))

(event `updateMinerSpeed`
  (for _array_element (`self.minersArray`)
    (set `/Game/Blueprints/BP_Miner.speed` (`/Game/Blueprints/BP_ClickerPlayer.minerSpeed` (`self.Player`)) _array_element)))

(event `updateMinerRest`
  (for _array_element (`self.minersArray`)
    (set `/Game/Blueprints/BP_Miner.rest` (`/Game/Blueprints/BP_ClickerPlayer.minerRest` (`self.Player`)) _array_element)))

(fn `activateLayer`
  (params (d1Index :type Integer))
  (bind _terrainlayers (`self.terrainLayers`))
  (for _index (range (`/Game/Blueprints/BP_LayersArray.d2Size` _terrainlayers))
    (bind _terrainobject (`/Game/Blueprints/BP_LayersArray.GetElement2D` _terrainlayers d1Index _index))
    (set `/Game/Blueprints/Layers/BP_TerrainCube.isActive` true _terrainobject)))

(fn `generateLayers`
  (locals (xValue :type "Float (double-precision)") (yValue :type "Float (double-precision)") (zValue :type "Float (double-precision)") (xIndex :type "Float (double-precision)"))
  (bind _terrainlayers (`self.terrainLayers`))
  (bind _d1size (`/Game/Blueprints/BP_LayersArray.d1Size` _terrainlayers))
  (set `local.zValue` (`KismetMathLibrary.Conv_IntToDouble` (* _d1size 100)))
  (for _index (range _d1size)
    (for _index_2 (range (`/Game/Blueprints/BP_LayersArray.d2Size` _terrainlayers))
      (bind _returnvalue (`|SpawnActorFromClass` (`|GetArrayItem` (`self.layerTypesArray`) _index) (`KismetMathLibrary.MakeTransform` (`KismetMathLibrary.MakeVector` (`local.xValue`) (`local.yValue`) (`local.zValue`))) "Undefined" "MultiplyWithRoot" null null))
      (`/Game/Blueprints/BP_LayersArray.SetElement2D` (`self.terrainLayers`) _index _index_2 _returnvalue)
      (bind _output_get (set `local.xValue` (+ (`local.xValue`) 100.0)))
      (if (> _output_get 400.0)
        (set `local.xValue` 0.0)
        (set `local.yValue` (+ (`local.yValue`) 100.0))))
    (set `local.zValue` (- (`local.zValue`) 100.0))
    (set `local.xValue` 0.0)
    (set `local.yValue` 0.0)))

(fn `UserConstructionScript`)